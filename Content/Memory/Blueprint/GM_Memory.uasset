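; GM_Memory is the game mode for a card-matching memory game, playing background music and judging pairs.
; OnCardClicked stores the first card in PrevCard, then compares its Type with the second card's.
; A match adds to Score, prints it and destroys both cards, while a mismatch immediately toggles both cards.
; PrevCard clears after each pair, and Test_map opens when Score reaches six.
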(event EventBeginPlay
  (Audio|PlaySound2D "/Game/Sound/dangdut-part-2-indonesian-music-4922.dangdut-part-2-indonesian-music-4922" 1.0 1.0 0.0 0 0))

(fn ConstructionScript)

(fn OnCardClicked
  (params (Card :type BP%20Card%20Object%20Reference))
  (if (Utilities|IsValid (Variables|Default|GetPrevCard))
    (if (Utilities|Enum|Equal(Enum) (Variables|/Game/Memory/Blueprint/BP_Card.BP_Card_C|GetType Card) (Variables|/Game/Memory/Blueprint/BP_Card.BP_Card_C|GetType (Variables|Default|GetPrevCard)))
      (bind _result (Math|Integer|IncrementInt (Variables|Default|GetScore))
        (:%20%20
          (bind _output_get (Variables|Default|SetScore _result))
          (Development|PrintString (Utilities|String|ToString(Integer) _output_get))
          (Actor|DestroyActor Card)
          (Actor|DestroyActor (Variables|Default|GetPrevCard))))
      (else
        (Default|ToggleCard Card)
        (Default|ToggleCard (Variables|Default|GetPrevCard))))
    (Variables|Default|SetPrevCard 0)
    (if (== (Variables|Default|GetScore) 6)
      (Game|OpenLevel(byName) "Test_map"))
    (else
      (Variables|Default|SetPrevCard Card))))