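; BP_Card is a clickable card for a memory game, with a face showing one of six types such as Genderuwo, Kuntilanak or Maung.
; The construction script sets the Verso material from the card's Type.
; Clicking a clickable card toggles its clickability and flips its root between 0 and 180 degrees of roll.
; After a short delay, it reports itself to GM_Memory through OnCardClicked.
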(event EventBeginPlay
  (bind _asgm_memory (Utilities|Casting|CastToGM_Memory (Game|GetGameMode)))
  (Variables|Default|SetAs%20GM%20Memory _asgm_memory))

(event MouseInput|EventActorOnClicked
  (params (ButtonPressed :type Key%20Structure :default "None"))
  (if (Variables|Default|GetisClickable)
    (CallFunction|ToggleCard)
    (Utilities|FlowControl|Delay 0.5)
    (Default|OnCardClicked (Variables|Default|GetAs%20GM%20Memory) self)))

(fn ConstructionScript
  (CallFunction|ChangeCardType))

(fn ChangeCardType
  (switch Utilities|FlowControl|Switch|SwitchonE_CardTypes (Variables|Default|GetType)
    (:NewEnumerator0
      (Rendering|Material|SetMaterial (Variables|Default|GetVerso) 0 "/Game/Images/Folklore/MI_Genderuwo.MI_Genderuwo"))
    (:NewEnumerator1
      (Rendering|Material|SetMaterial (Variables|Default|GetVerso) 0 "/Game/Images/Folklore/MI_Kuntilanak.MI_Kuntilanak"))
    (:NewEnumerator2
      (Rendering|Material|SetMaterial (Variables|Default|GetVerso) 0 "/Game/Images/Folklore/MI_LoroJonggrang.MI_LoroJonggrang"))
    (:NewEnumerator3
      (Rendering|Material|SetMaterial (Variables|Default|GetVerso) 0 "/Game/Images/Folklore/MI_Maung.MI_Maung"))
    (:NewEnumerator4
      (Rendering|Material|SetMaterial (Variables|Default|GetVerso) 0 "/Game/Images/Folklore/MI_Pennangalang.MI_Pennangalang"))
    (:NewEnumerator5
      (Rendering|Material|SetMaterial (Variables|Default|GetVerso) 0 "/Game/Images/Folklore/MI_SundelBolong.MI_SundelBolong"))))

(fn ToggleCard
  (Variables|Default|SetisClickable (not (Variables|Default|GetisClickable)))
  (if (== (.roll (Transformation|GetWorldRotation (Variables|Default|GetDefaultSceneRoot))) 0.0)
    (Transformation|SetRelativeRotation (Variables|Default|GetDefaultSceneRoot) (Math|Rotator|MakeRotator 1.8e+02 0.0 0.0) false false)
    (else
      (Transformation|SetRelativeRotation (Variables|Default|GetDefaultSceneRoot) (Math|Rotator|MakeRotator 0.0 0.0 0.0) false false))))