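; Player Blueprint that caches the game mode and handles toggling the game's pause menu.
; On BeginPlay it casts the game mode to BP_GameMode and stores the reference, which this graph does not use further.
; A P debug key event flips IsGamePaused, either creating a WB_Pause widget with Game-and-UI input and pausing, or removing it, unpausing and restoring game-only input.
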(event EventBeginPlay
  (bind _asbp_game_mode (Utilities|Casting|CastToBP_GameMode (Game|GetGameMode)))
  (Variables|Default|SetAs%20BP%20Game%20Mode _asbp_game_mode))

(event Input|KeyboardEvents|DebugKeyP
  (params (Key :type Key%20Structure :default "None") (ActionValue :type Input%20Action%20Value%20Structure))
  (bind _returnvalue (Game|GetPlayerController 0))
  ;[0 0 0] Game Pause
  (:Pressed
    (if (not (Variables|Default|GetIsGamePaused))
      (Variables|Default|SetIsGamePaused true)
      (bind _returnvalue_2 (UserInterface|CreateWidget "/Game/Widgets/WB_Pause.WB_Pause_C" _returnvalue))
      (bind _output_get (Variables|Default|SetPause _returnvalue_2))
      (UserInterface|Viewport|AddtoViewport _output_get 0)
      (Input|SetInputModeGameandUI _returnvalue 0 "DoNotLock" true false)
      (Game|SetGamePaused true)
      (else
        (Variables|Default|SetIsGamePaused false)
        (Widget|RemovefromParent (Variables|Default|GetPause))
        (Game|SetGamePaused false)
        (Input|SetInputModeGameOnly 0 false)))))

(fn ConstructionScript)